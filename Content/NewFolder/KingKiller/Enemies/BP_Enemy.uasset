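; BP_Enemy is an enemy that chases the player on sight and is destroyed when its HP runs out.
; PawnSensing triggers an AI MoveTo toward any seen pawn that implements the BI_IAmThePlayer interface, avoiding a cast to the player class.
; GetDamage subtracts from HP, prints the remaining value and calls Die at zero or below, which destroys the actor.
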(event `/Game/NewFolder/KingKiller/Interfaces/BI_IAmAlive.Die`
  (`self.K2_DestroyActor`))

(event `self.ReceiveEndPlay`
  (params (EndPlayReason :type "EEndPlayReason Enum" :default "Destroyed")))

(event `/Game/NewFolder/KingKiller/Interfaces/BI_IAmAlive.GetDamage`
  (params (Damage :type "Float (double-precision)"))
  (bind _output_get (set `self.HP` (- (`self.HP`) Damage)))
  (`KismetSystemLibrary.PrintString` (`KismetStringLibrary.Conv_DoubleToString` _output_get) true true (struct :`G` 0.66 :`B` 1.0 :`A` 1.0) _output_get)
  (if (<= _output_get 0.0)
    (`self.Die`)))

(event `self.PawnSensing.OnSeePawn`
  (params (Pawn :type "Pawn Object Reference"))
  (if (`KismetSystemLibrary.DoesImplementInterface` Pawn "/Game/NewFolder/KingKiller/Interfaces/BI_IAmThePlayer.BI_IAmThePlayer_C")
    (`|AIMoveTo` self (0.0 0.0 0.0) Pawn)))

(fn `UserConstructionScript`)