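; BP_KingKillerPawn is a pawn that spawns copies of itself and launches them as physics projectiles along its capsule's forward vector.
; Each copy gets capsule physics simulation and a large impulse.
; Space fires immediately, while Tick repeats the shot through a two-second Delay whenever the game instance reports debugging.
; ControllerClick clears that debug flag; ControllerDebugClick only casts, leaving the call that sets it unconnected.
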(event `InputAction|ControllerDebugClick`
  (params (Key :type "Key Structure"))
  (:`Pressed`
    (cast `/Game/NewFolder/BP_MyGameInstance` (`GameplayStatics.GetGameInstance`))))

(event `self.ReceiveTick`
  (params (DeltaSeconds :type "Float (single-precision)"))
  (bind _asbp_my_game_instance (cast `/Game/NewFolder/BP_MyGameInstance` (`GameplayStatics.GetGameInstance`)))
  (if (`MyGameInstance.IsDebugging` _asbp_my_game_instance)
    (`KismetSystemLibrary.Delay` 2.0)
    (bind _returnvalue (`|SpawnActorFromClass` "BP_KingKillerPawn_C" (`self.GetTransform`) "AdjustIfPossibleButAlwaysSpawn" "MultiplyWithRoot" null null :!label _label))
    (bind _capsulecomponent (`Character.CapsuleComponent` _returnvalue))
    (`PrimitiveComponent.SetSimulatePhysics` _capsulecomponent true)
    (`PrimitiveComponent.AddImpulse` _capsulecomponent (* (`SceneComponent.GetForwardVector` (`self.CapsuleComponent`)) 1000000.0) "None" false)))

(event `Key|SpaceBar`
  (params (Key :type "Key Structure"))
  (:`Pressed`
    (goto _label)))

(event `InputAction|ControllerClick`
  (params (Key :type "Key Structure"))
  (:`Pressed`
    (bind _asbp_my_game_instance (cast `/Game/NewFolder/BP_MyGameInstance` (`GameplayStatics.GetGameInstance`)))
    (`MyGameInstance.SetIsDebugging` _asbp_my_game_instance false)))

(fn `UserConstructionScript`)