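; Player character for the KingKiller mode, with Enhanced Input movement, look, jump, sprint and shooting.
; The construction script loads health, speeds, jump velocity and mesh by unit type, then reads damage from the child-actor weapon before applying its type.
; Shooting sphere-traces from the spawn point to one unit ahead of the camera and sends damage to the hit actor.
; Physics-bullet spawning and debug-toggle logic are present but disconnected.
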(event `self.ReceiveBeginPlay`
  (bind _asplayer_controller (cast `PlayerController` (`self.GetController`)))
  (bind _returnvalue (pcsubsystem `EnhancedInputLocalPlayerSubsystem` _asplayer_controller))
  (`/Engine/EditorBlueprintResources/StandardMacros.IsValid` _returnvalue
    (:`Is Valid`
      (`EnhancedInputSubsystemInterface.AddMappingContext` _returnvalue "/Game/NewFolder/KingKiller/Inputs/IMap_KingKiller.IMap_KingKiller" 0 (struct)))))

(event `InputAction|ControllerDebugClick`
  (params (Key :type "Key Structure")))

(event `InputAction|ControllerClick`
  (params (Key :type "Key Structure")))

(event `EnhancedInput|/Game/NewFolder/KingKiller/Inputs/IA_Jump`
  (params (ActionValue :type Boolean) (ElapsedSeconds :type "Float (double-precision)") (TriggeredSeconds :type "Float (double-precision)") (InputAction :type "InputAction Object Reference" :default "/Game/NewFolder/KingKiller/Inputs/IA_Jump.IA_Jump"))
  ;[0 0.03245 0.15 0.5] Jumping
  (:`Triggered`
    (`self.Jump`))
  (:`Completed`
    (`self.StopJumping`)))

(event `EnhancedInput|/Game/NewFolder/KingKiller/Inputs/IA_Walk`
  (params (ActionValue :type "Vector2D Structure") (ElapsedSeconds :type "Float (double-precision)") (TriggeredSeconds :type "Float (double-precision)") (InputAction :type "InputAction Object Reference" :default "/Game/NewFolder/KingKiller/Inputs/IA_Walk.IA_Walk"))
  ;[0.15 0 0 0.5] Walk
  (:`Triggered`
    (`self.AddMovementInput` (`self.GetActorRightVector`) ActionValue_X)
    (`self.AddMovementInput` (`self.GetActorForwardVector`) ActionValue_Y)))

(event `EnhancedInput|/Game/NewFolder/KingKiller/Inputs/IA_Look`
  (params (ActionValue :type "Vector2D Structure") (ElapsedSeconds :type "Float (double-precision)") (TriggeredSeconds :type "Float (double-precision)") (InputAction :type "InputAction Object Reference" :default "/Game/NewFolder/KingKiller/Inputs/IA_Look.IA_Look"))
  ;[0 0.15 0.03213 0.5] Looking
  (:`Triggered`
    (`self.AddControllerYawInput` ActionValue_X)
    (`self.AddControllerPitchInput` ActionValue_Y)))

(event `EnhancedInput|/Game/NewFolder/KingKiller/Inputs/IA_ShootWeapon`
  (params (ActionValue :type Boolean) (ElapsedSeconds :type "Float (double-precision)") (TriggeredSeconds :type "Float (double-precision)") (InputAction :type "InputAction Object Reference" :default "/Game/NewFolder/KingKiller/Inputs/IA_ShootWeapon.IA_ShootWeapon"))
  (bind _camera (`self.Camera`))
  (:`Triggered`
    (bind _outhit (`KismetSystemLibrary.SphereTraceSingle` :`Start` (`SceneComponent.K2_GetComponentLocation` (`self.Spawnpoint`)) :`End` (+ (`SceneComponent.K2_GetComponentLocation` _camera) (`SceneComponent.GetForwardVector` _camera)) :`Radius` 150.0 :`TraceChannel` "TraceTypeQuery5" :`DrawDebugType` "ForDuration"))
    (message `/Game/NewFolder/KingKiller/Interfaces/BI_IAmAlive.GetDamage` (`.HitActor` (`GameplayStatics.BreakHitResult` _outhit)) (`self.WeaponDamage`))))

(event `EnhancedInput|/Game/NewFolder/KingKiller/Inputs/IA_Sprint`
  (params (ActionValue :type Boolean) (ElapsedSeconds :type "Float (double-precision)") (TriggeredSeconds :type "Float (double-precision)") (InputAction :type "InputAction Object Reference" :default "/Game/NewFolder/KingKiller/Inputs/IA_Sprint.IA_Sprint"))
  (:`Triggered`
    (set `CharacterMovementComponent.MaxWalkSpeed` (`self.SprintWalkSpeed`) (`self.CharacterMovement`)))
  (:`Completed`
    (set `CharacterMovementComponent.MaxWalkSpeed` (`self.NormalWalkSpeed`) (`self.CharacterMovement`))))

(fn `UserConstructionScript`
  (bind _unitdata (`/Game/NewFolder/KingKiller/BFL_KingKiller.GetKingKillerUnitDataType` (`self.UnitType`)))
  (bind (_unittype _mesh _animationblueprint _hp _normalwalkingspeed _sprintingspeed _jumpheight) (break `/Game/NewFolder/KingKiller/S_KingKillerData` _unitdata))
  (set `self.HP` _hp)
  (set `self.NormalWalkSpeed` _normalwalkingspeed)
  (set `self.SprintWalkSpeed` _sprintingspeed)
  (set `CharacterMovementComponent.JumpZVelocity` _jumpheight (`self.CharacterMovement`))
  (`SkeletalMeshComponent.SetSkeletalMeshAsset` (`self.Mesh`) _mesh)
  (bind _asbp_weapon (cast `/Game/NewFolder/KingKiller/Weapon/BP_Weapon` (`ChildActorComponent.ChildActor` (`self.Weapon`))))
  (set `self.WeaponDamage` (`/Game/NewFolder/KingKiller/Weapon/BP_Weapon.Damage` _asbp_weapon))
  (bind _output_get (set `/Game/NewFolder/KingKiller/Weapon/BP_Weapon.WeaponType` (`self.Weapontype`) _asbp_weapon))
  (`/Game/NewFolder/KingKiller/Weapon/BP_Weapon.ChangeWeaponTypeAndAnimation` _asbp_weapon _output_get))